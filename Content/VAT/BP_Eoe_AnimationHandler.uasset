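; Actor that registers vertex animation texture (VAT) frame ranges for each unit type with a subsystem at BeginPlay.
; It reads every DT_Animations row and converts animation length and frame rate into a rounded frame count.
; The PrevOfType map keeps a running frame total per mesh name, so each mesh's animations get consecutive start and end frames in table row order.
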(event `Add Animations`
  (bind _prevoftype (`self.PrevOfType`))
  (bind _outrownames (`DataTableFunctionLibrary.GetDataTableRowNames` null))
  (for _array_element _outrownames
    (bind _returnvalue (`|GetDataTableRow` "/Game/VAT/DT_Animations.DT_Animations" _array_element)
      (:`then`
        (bind (_mesh _type) (break `/Game/VAT/ST_AnimationStruct` _returnvalue))
        (bind _returnvalue_2 (`KismetSystemLibrary.GetObjectName` _mesh))
        (if (`BlueprintMapLibrary.Map_Contains` (`self.PrevOfType`) _returnvalue_2)
          (bind _value (`BlueprintMapLibrary.Map_Find` _prevoftype _returnvalue_2))
          (bind (_mesh_2 _type_2 _animation _playrate _framerate) (break `/Game/VAT/ST_AnimationStruct` _returnvalue))
          (bind _returnvalue_3 (`KismetMathLibrary.Conv_IntToDouble` (`KismetMathLibrary.Round` (* (`AnimationAsset.GetPlayLength` _animation) _framerate))))
          (bind _returnvalue_4 (+ _value _returnvalue_3))
          (`self.AddUnitTypeAnimTimings` (subsystem `Subsystem` null) _returnvalue_2 _type (+ _value 1.0) (+ _returnvalue_4 0.0))
          (`BlueprintMapLibrary.Map_Add` _prevoftype _returnvalue_2 _returnvalue_4)
          (else
            (`BlueprintMapLibrary.Map_Add` (`self.PrevOfType`) (`KismetSystemLibrary.GetObjectName` _mesh_2) _returnvalue_3)
            (`self.AddUnitTypeAnimTimings` (subsystem `Subsystem` null) _returnvalue_2 _type 0.0 (- _returnvalue_3 1.0))))))))

(event `self.ReceiveBeginPlay`
  (`self.Add Animations`))

(fn `UserConstructionScript`)