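; BP_Ee_PlayerController is a player controller that turns Enhanced Input actions into calls on the possessed BP_BasePlayer pawn.
; On BeginPlay it adds the third-person mapping context, caches the pawn, passes it the PlayerIndex and binds to possession changes to refresh both.
; Move, jump, camera turn and mode change are forwarded to that cached pawn.
; Only camera turn checks pawn validity, and it also debug-prints an input axis.
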(event `TPS Mapping Context`
  (message `EnhancedInputSubsystemInterface.AddMappingContext` (subsystem `EnhancedInputLocalPlayerSubsystem`) "/Game/EE/Controls/IMC_ThirdPerson.IMC_ThirdPerson" 0 (struct)))

(event `EnhancedInput|/Game/EE/Controls/IA_TurnCamera`
  (params (ActionValue :type "Vector2D Structure") (ElapsedSeconds :type "Float (double-precision)") (TriggeredSeconds :type "Float (double-precision)") (InputAction :type "InputAction Object Reference" :default "/Game/EE/Controls/IA_TurnCamera.IA_TurnCamera"))
  (bind _currentcontrolledpawn (`self.CurrentControlledPawn`))
  (:`Triggered`
    (`/Engine/EditorBlueprintResources/StandardMacros.IsValid` _currentcontrolledpawn
      (:`Is Valid`
        (`/Game/EE/ActorRepresentations/BP_BasePlayer.CameraMoveTPSFromPC` _currentcontrolledpawn ActionValue_X ActionValue_Y)
        (`KismetSystemLibrary.PrintString` (`KismetStringLibrary.Conv_DoubleToString` ActionValue_X))))))

(event `EnhancedInput|/Game/EE/Controls/IA_ChangeMode`
  (params (ActionValue :type Boolean) (ElapsedSeconds :type "Float (double-precision)") (TriggeredSeconds :type "Float (double-precision)") (InputAction :type "InputAction Object Reference" :default "/Game/EE/Controls/IA_ChangeMode.IA_ChangeMode"))
  (:`Triggered`
    (`/Game/EE/ActorRepresentations/BP_BasePlayer.PlayerTPSCamera` (`self.CurrentControlledPawn`))))

(event `EnhancedInput|/Game/EE/Controls/IA_Move`
  (params (ActionValue :type "Vector2D Structure") (ElapsedSeconds :type "Float (double-precision)") (TriggeredSeconds :type "Float (double-precision)") (InputAction :type "InputAction Object Reference" :default "/Game/EE/Controls/IA_Move.IA_Move"))
  (:`Triggered`
    (`/Game/EE/ActorRepresentations/BP_BasePlayer.Movement Input From PC` (`self.CurrentControlledPawn`) ActionValue InputAction)))

(event `EnhancedInput|/Game/EE/Controls/IA_Jump`
  (params (ActionValue :type Boolean) (ElapsedSeconds :type "Float (double-precision)") (TriggeredSeconds :type "Float (double-precision)") (InputAction :type "InputAction Object Reference" :default "/Game/EE/Controls/IA_Jump.IA_Jump"))
  (bind _currentcontrolledpawn (`self.CurrentControlledPawn`))
  (:`Ongoing`
    (`/Game/EE/ActorRepresentations/BP_BasePlayer.FromPCJump` _currentcontrolledpawn))
  (:`Canceled`
    (`/Game/EE/ActorRepresentations/BP_BasePlayer.FromPCStopJump` _currentcontrolledpawn)))

(event `self.ReceiveBeginPlay`
  (`self.TPS Mapping Context`)
  (bind _asbp_base_player (cast `/Game/EE/ActorRepresentations/BP_BasePlayer` (`self.K2_GetPawn`)))
  (set `self.CurrentControlledPawn` _asbp_base_player)
  (add `self.OnPossessedPawnChanged` (delegate `OnPossessedPawnChanged_Event`))
  (set `/Game/EE/ActorRepresentations/BP_BasePlayer.Player Index` (`self.Player Index`) (`self.CurrentControlledPawn`) :!label _label))

(event `OnPossessedPawnChanged_Event` :!signature `self.OnPossessedPawnChanged`
  (params (OldPawn :type "Pawn Object Reference") (NewPawn :type "Pawn Object Reference"))
  (bind _asbp_base_player (cast `/Game/EE/ActorRepresentations/BP_BasePlayer` NewPawn))
  (set `self.CurrentControlledPawn` _asbp_base_player)
  (goto _label))

(fn `UserConstructionScript`)