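; BP_HighRep is an actor representation Blueprint that scales its tick rate by its distance from the player character.
; Tick runs the parent logic, then accumulates delta time until a check interval elapses.
; At each check it divides the player distance by a reference distance, subtracts an offset, clamps the result between zero and one, and passes it to SetTickrate.
; BeginPlay and construction only call the parent.
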(event `self.ReceiveBeginPlay`
  (`parent.ReceiveBeginPlay`))

(event `self.ReceiveTick`
  (params (DeltaSeconds :type "Float (single-precision)"))
  (`parent.ReceiveTick` DeltaSeconds)
  (bind _output_get (set `self.TickrateCheckCur` (+ DeltaSeconds (`self.TickrateCheckCur`))))
  (if (>= _output_get (`self.TickrateCheckInterval`))
    (`self.Set Tickrate` self (`KismetMathLibrary.FClamp` (- (/ (`self.GetDistanceTo` (`GameplayStatics.GetPlayerCharacter` 0) self) (`self.DistToCheck`)) (`self.OffsetTimes`))))
    (set `self.TickrateCheckCur` 0.0)))

(fn `UserConstructionScript`
  (`parent.UserConstructionScript`))